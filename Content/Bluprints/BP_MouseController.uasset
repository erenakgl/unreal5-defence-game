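; Player controller that turns the mouse cursor's world position into movement updates for the player's blocker (BP_PlayerLocker).
; On BeginPlay it finds the blocker and GameCamera in the level, switches the view to that camera, disables mouse capture and adds the game screen widget.
; Each Tick a complex WorldStatic trace under the cursor sends the hit location to the blocker, ignoring hits on the blocker itself.
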(event `self.ReceiveBeginPlay`
  ;[1 1 1] Begin
  (`|ExecutionSequence`
    (:`then_0`
      (bind _returnvalue (`GameplayStatics.GetActorOfClass` "/Game/Bluprints/BP_PlayerLocker.BP_PlayerLocker_C"))
      (set `self.PlayerBlocker` _returnvalue))
    (:`then_1`
      (bind _returnvalue_2 (`GameplayStatics.GetActorOfClass` "/Game/Bluprints/GameCamera.GameCamera_C"))
      (bind _output_get (set `self.Game Camera` _returnvalue_2))
      (`self.SetViewTargetWithBlend` _output_get))
    (:`then_2`
      (`GameplayStatics.SetViewportMouseCaptureMode` "NoCapture"))
    (:`then_3`
      (bind _returnvalue_3 (`|CreateWidget` "/Game/Bluprints/UMG/WB_GameScreen.WB_GameScreen_C"))
      (`UserWidget.AddToViewport` _returnvalue_3 0))))

(event `self.ReceiveTick`
  (params (DeltaSeconds :type "Float (single-precision)"))
  (bind (_hitresult _returnvalue) (`self.GetHitResultUnderCursorForObjects` (`|MakeArray` "ObjectTypeQuery1" :!type "EObjectTypeQuery Enum")))
  (bind (_bblockinghit _binitialoverlap _time _distance _location _impactpoint _normal _impactnormal _physmat _hitactor) (`GameplayStatics.BreakHitResult` _hitresult))
  (if _returnvalue
    (if (!= (`GameplayStatics.GetObjectClass` _hitactor) "/Game/Bluprints/BP_PlayerLocker.BP_PlayerLocker_C")
      (bind _output_get (set `self.MouseLocation` _location))
      (message `/Game/Bluprints/BPI_MainGameplay.UpdateLocationFromMouse` (`self.PlayerBlocker`) _output_get))))

(fn `UserConstructionScript`)