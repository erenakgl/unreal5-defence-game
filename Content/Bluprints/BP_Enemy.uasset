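; BP_Enemy is an AI-driven enemy that advances along a straight path toward a win zone.
; On BeginPlay it finds the GameManager and issues an AIMoveTo 2000 units along +Y from its spawn location.
; Hitting a BP_PlayerLocker while Killable reports EnemyStopped, halts movement by retargeting its current location, then destroys it after a short delay.
; Overlapping an EnemyWinZone reports EnemyWon to the GameManager and destroys it after a delay.
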(event `OnStop`
  (`|AIMoveTo` self (`self.K2_GetActorLocation`) null))

(event `self.ReceiveBeginPlay`
  (`|ExecutionSequence`
    (:`then_0`
      ;[1 1 1] Game Manager Set
      (bind _returnvalue (`GameplayStatics.GetActorOfClass` "/Game/Bluprints/GameManager.GameManager_C"))
      (set `self.Game Manager` _returnvalue))
    (:`then_1`
      ;[1 1 1] AI Movement
      (`parent.ReceiveBeginPlay`)
      (`|AIMoveTo` self (+ (`self.K2_GetActorLocation`) (0.0 2000.0 0.0)) null))))

(event `self.ReceiveHit`
  (params (MyComp :type "PrimitiveComponent Object Reference") (Other :type "Actor Object Reference") (OtherComp :type "PrimitiveComponent Object Reference") (bSelfMoved :type Boolean) (HitLocation :type "Vector Structure") (HitNormal :type "Vector Structure") (NormalImpulse :type "Vector Structure") (Hit :type "HitResult Structure (by ref)"))
  ;[1 1 1] On Stop
  (if (== (`GameplayStatics.GetObjectClass` (`.HitActor` (`GameplayStatics.BreakHitResult` Hit))) "/Game/Bluprints/BP_PlayerLocker.BP_PlayerLocker_C")
    (if (`self.Killable`)
      (`/Game/Bluprints/GameManager.EnemyStopped` (`self.Game Manager`))
      (`self.OnStop`)
      (`KismetSystemLibrary.Delay` 0.5)
      (`self.K2_DestroyActor`))))

(event `self.ReceiveActorBeginOverlap`
  (params (OtherActor :type "Actor Object Reference"))
  (if (== (`GameplayStatics.GetObjectClass` OtherActor) "/Game/Bluprints/EnemyWinZone.EnemyWinZone_C")
    (`/Game/Bluprints/GameManager.EnemyWon` (`self.Game Manager`))
    (`KismetSystemLibrary.Delay` 2.0)
    (`self.K2_DestroyActor`)))

(fn `UserConstructionScript`
  (`parent.UserConstructionScript`))