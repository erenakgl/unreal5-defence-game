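; BP_PlayerLocker is an actor that follows the mouse along X, confined between the goal posts in the level.
; On BeginPlay it gathers every BP_GoalPost location and caches the minimum and maximum X as bounds.
; UpdateLocationfromMouse moves the actor to the clamped mouse X, keeping its Y and Z, until the GameOver event sets a flag that freezes it.
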(event `self.ReceiveBeginPlay`
  (bind _goalzone_x (`self.GoalZone X`))
  (`|ExecutionSequence`
    (:`then_0`
      (bind _outactors (`GameplayStatics.GetAllActorsOfClass` "/Game/Bluprints/BP_GoalPost.BP_GoalPost_C"))
      (for _array_element _outactors
        (bind _returnvalue (`self.K2_GetActorLocation` _array_element))
        (`KismetArrayLibrary.Array_Add` (`self.GoalZones`) _returnvalue)
        (`KismetArrayLibrary.Array_Add` (`self.GoalZone X`) (.x _returnvalue))))
    (:`then_1`
      (set `self.Max X` (`.MaxValue` (`KismetMathLibrary.MaxOfFloatArray` _goalzone_x))))
    (:`then_2`
      (set `self.Min X` (`.MinValue` (`KismetMathLibrary.MinOfFloatArray` _goalzone_x))))))

(event `/Game/Bluprints/BPI_MainGameplay.UpdateLocationFromMouse`
  (params (MouseLocation :type "Vector Structure"))
  (if (not (`self.Game Over`))
    (`self.K2_SetActorLocation` (`KismetMathLibrary.MakeVector` (`KismetMathLibrary.FClamp` (.x MouseLocation) (`self.Min X`) (`self.Max X`)) (.y (`self.K2_GetActorLocation`)) (.z (`self.K2_GetActorLocation`))))))

(event `/Game/Bluprints/BPI_MainGameplay.GameOver`
  (set `self.Game Over` true))

(fn `UserConstructionScript`)